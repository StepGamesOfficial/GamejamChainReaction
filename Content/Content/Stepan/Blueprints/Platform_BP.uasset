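; Platform actor that can optionally let the player jump up through it from below.
; On Tick, when CanJumpThrough is set, it compares player and platform heights, switching the Cube's response to the player capsule's channel to Block well above and Ignore below.
; Otherwise it sets Block once through a DoOnce.
; The construction script labels a TextRender with whether the platform can be jumped through.
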(event EventBeginPlay)

(event Collision|EventActorBeginOverlap
  (params (OtherActor :type Actor%20Object%20Reference)))

(event EventTick
  (params (DeltaSeconds :type Float%20%28single-precision%29))
  (bind _returnvalue (Game|GetPlayerCharacter 0))
  (bind _returnvalue_2 (Game|GetPlayerController 0))
  (bind _cube (Variables|Default|GetCube))
  (bind _returnvalue_3 (Pawn|GetControlledPawn _returnvalue_2))
  (bind _capsulecomponent (Variables|/Script/Engine.Character|GetCapsuleComponent _returnvalue))
  (bind _returnvalue_4 (Collision|GetCollisionObjectType _capsulecomponent))
  (if (Variables|Default|GetCanJumpThrough)
    (if (> (.z (Transformation|GetActorLocation _returnvalue_3)) (+ (.z (Transformation|GetActorLocation)) 9e+01))
      (Collision|SetCollisionResponsetoChannel _cube _returnvalue_4 "ECR_Block" :!label _label)
      (elif (< (.z (Transformation|GetActorLocation _returnvalue_3)) (.z (Transformation|GetActorLocation)))
        (Collision|SetCollisionResponsetoChannel _cube _returnvalue_4 "ECR_Ignore")))
    (else
      (Utilities|FlowControl|DoOnce false
        (:Completed
          (goto _label))))))

(fn ConstructionScript
  (Rendering|Components|TextRender|SetText (Variables|Default|GetTextRender) (select (Variables|Default|GetCanJumpThrough) (Utilities|Text|MakeLiteralText "Can jump through") (Utilities|Text|MakeLiteralText "Can NOT jump through"))))