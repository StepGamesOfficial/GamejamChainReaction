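; Player character base for Water and Fire variants, with sideways movement, jumping, possession switching and projectile shooting.
; A BeginPlay loop drives timeline-based limb swinging while walking, then eases the body to neutral once on stopping.
; A/D turn the body and aim Arrow1, the spawn point for E's element-specific projectile.
; Tab (when not falling) or ForceSwitch possesses the other element's character and adds its UI, with Tab clearing widgets first.
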(event Custom|ForceSwitch
  (bind _returnvalue (Game|GetPlayerController 0))
  (switch Utilities|FlowControl|Switch|SwitchonPlayerType_Enum (Variables|Default|GetType)
    (:NewEnumerator0
      (bind _outactors (Actor|GetAllActorsOfClass "/Game/Content/Stepan/Blueprints/PlayerCharacter_BP_Fire.PlayerCharacter_BP_Fire_C"))
      (Pawn|Possess _returnvalue (Utilities|Array|Get(acopy) _outactors))
      (bind _returnvalue_2 (UserInterface|CreateWidget "/Game/Content/Nowster/FireUI.FireUI_C" _returnvalue))
      (UserInterface|Viewport|AddtoViewport _returnvalue_2 0))
    (:NewEnumerator1
      (bind _outactors_2 (Actor|GetAllActorsOfClass "/Game/Content/Stepan/Blueprints/PlayerCharacter_BP_Water.PlayerCharacter_BP_Water_C"))
      (Pawn|Possess _returnvalue (Utilities|Array|Get(acopy) _outactors_2))
      (bind _returnvalue_3 (UserInterface|CreateWidget "/Game/Content/Nowster/WaterUI.WaterUI_C" _returnvalue))
      (UserInterface|Viewport|AddtoViewport _returnvalue_3 0))))

(event Collision|EventActorBeginOverlap
  (params (OtherActor :type Actor%20Object%20Reference)))

(event EventTick
  (params (DeltaSeconds :type Float%20%28single-precision%29)))

(event EventBeginPlay
  (if (Variables|Default|GetIsWalking) :!label _label
    (Utilities|FlowControl|Sequence
      (:then_0
        (bind _alpha (Timeline|Timeline_0 PlayFromStart)
          (:Update
            (Transformation|SetRelativeRotation (Variables|Default|Getwatergirl_Leg) (Math|Rotator|Lerp(Rotator) "-20.000000, 0, 0" "20.000000, 0, 0" _alpha true) false false)
            (Transformation|SetRelativeRotation (Variables|Default|Getwatergirl_Leg2) (Math|Rotator|Lerp(Rotator) "20.000000, 0, 0" "-20.000000, 0, 0" _alpha true) false false))
          (:Finished
            (goto _label))))
      (:then_1
        (goto _label_2 Reset)))
    (else
      (Utilities|FlowControl|Sequence
        (:then_0
          (Utilities|FlowControl|Delay 0.2)
          (goto _label))
        (:then_1
          (Timeline|Timeline_0 Stop))
        (:then_2
          (Utilities|FlowControl|DoOnce false :!label _label_2
            (:Completed
              (Variables|Default|SetGoalRotation "0, 0, 0")
              (Variables|Default|SetLastRotation (Variables|/Script/Engine.SceneComponent|GetRelativeRotation (Variables|Default|Getwatergirl_Drop)))
              (bind _alpha_2 (Timeline|Rotate PlayFromStart)
                (:Update
                  (Transformation|SetRelativeRotation (Variables|Default|Getwatergirl_Drop) (Math|Rotator|Lerp(Rotator) (Variables|Default|GetLastRotation) (Variables|Default|GetGoalRotation) _alpha_2 true) false false))
                (:Finished
                  (Transformation|SetRelativeRotation (Variables|Default|Getwatergirl_Leg) "0, 0, 0" false false)
                  (Transformation|SetRelativeRotation (Variables|Default|Getwatergirl_Leg2) "0, 0, 0" false false))))))))))

(event Input|AxisEvents|InputAxisMoveRight
  (params (AxisValue :type Float%20%28single-precision%29))
  (Pawn|Input|AddMovementInput (Transformation|GetActorRightVector) AxisValue false)
  (Variables|Default|SetIsWalking (!= AxisValue 0.0)))

(event Input|KeyboardEvents|SpaceBar
  (params (Key :type Key%20Structure :default "None"))
  (:Pressed
    (Character|Jump)))

(event Input|KeyboardEvents|Tab
  (params (Key :type Key%20Structure :default "None"))
  (bind _returnvalue (Game|GetPlayerController 0))
  (:Pressed
    (if (not (AI|Components|NavMovement|IsFalling (Variables|Character|GetCharacterMovement)))
      (Viewport|RemoveAllWidgets)
      (switch Utilities|FlowControl|Switch|SwitchonPlayerType_Enum (Variables|Default|GetType)
        (:NewEnumerator0
          (bind _outactors (Actor|GetAllActorsOfClass "/Game/Content/Stepan/Blueprints/PlayerCharacter_BP_Fire.PlayerCharacter_BP_Fire_C"))
          (Pawn|Possess _returnvalue (Utilities|Array|Get(acopy) _outactors))
          (bind _returnvalue_2 (UserInterface|CreateWidget "/Game/Content/Nowster/FireUI.FireUI_C" _returnvalue))
          (UserInterface|Viewport|AddtoViewport _returnvalue_2 0))
        (:NewEnumerator1
          (bind _outactors_2 (Actor|GetAllActorsOfClass "/Game/Content/Stepan/Blueprints/PlayerCharacter_BP_Water.PlayerCharacter_BP_Water_C"))
          (Pawn|Possess _returnvalue (Utilities|Array|Get(acopy) _outactors_2))
          (bind _returnvalue_3 (UserInterface|CreateWidget "/Game/Content/Nowster/WaterUI.WaterUI_C" _returnvalue))
          (UserInterface|Viewport|AddtoViewport _returnvalue_3 0))))))

(event Input|KeyboardEvents|E
  (params (Key :type Key%20Structure :default "None"))
  (bind _arrow1 (Variables|Default|GetArrow1))
  (bind _returnvalue (Transformation|GetWorldTransform _arrow1))
  (:Pressed
    (switch Utilities|FlowControl|Switch|SwitchonPlayerType_Enum (Variables|Default|GetType)
      (:NewEnumerator0
        (Game|SpawnActorfromClass "/Game/Content/Stepan/Blueprints/Projectile_Water.Projectile_Water_C" (Math|Transform|MakeTransform (.location _returnvalue) (.rotation _returnvalue) "0.450000,0.450000,0.450000") "Undefined" 0 0))
      (:NewEnumerator1
        (Game|SpawnActorfromClass "/Game/Content/Stepan/Blueprints/Projectile_Fire.Projectile_Fire_C" (Math|Transform|MakeTransform (.location _returnvalue) (.rotation _returnvalue) "0.450000,0.450000,0.450000") "Undefined" 0 0)))))

(event Input|KeyboardEvents|D
  (params (Key :type Key%20Structure :default "None"))
  (:Pressed
    (Transformation|SetRelativeRotation (Variables|Default|GetArrow1) (Math|Rotator|MakeRotator 0.0 0.0 2.7e+02) false false)
    (Variables|Default|SetGoalRotation "0,-90.000000, 0")
    (Variables|Default|SetLastRotation (Variables|/Script/Engine.SceneComponent|GetRelativeRotation (Variables|Default|Getwatergirl_Drop)))
    (bind _alpha (Timeline|Rotate PlayFromStart)
      (:Update
        (Transformation|SetRelativeRotation (Variables|Default|Getwatergirl_Drop) (Math|Rotator|Lerp(Rotator) (Variables|Default|GetLastRotation) (Variables|Default|GetGoalRotation) _alpha true) false false))
      (:Finished
        (Transformation|SetRelativeRotation (Variables|Default|Getwatergirl_Leg) "0, 0, 0" false false)
        (Transformation|SetRelativeRotation (Variables|Default|Getwatergirl_Leg2) "0, 0, 0" false false)))))

(event Input|KeyboardEvents|A
  (params (Key :type Key%20Structure :default "None"))
  (:Pressed
    (Transformation|SetRelativeRotation (Variables|Default|GetArrow1) (Math|Rotator|MakeRotator 0.0 0.0 9e+01) false false)
    (Variables|Default|SetGoalRotation "0,90.000000, 0")
    (Variables|Default|SetLastRotation (Variables|/Script/Engine.SceneComponent|GetRelativeRotation (Variables|Default|Getwatergirl_Drop)))
    (bind _alpha (Timeline|Rotate PlayFromStart)
      (:Update
        (Transformation|SetRelativeRotation (Variables|Default|Getwatergirl_Drop) (Math|Rotator|Lerp(Rotator) (Variables|Default|GetLastRotation) (Variables|Default|GetGoalRotation) _alpha true) false false))
      (:Finished
        (Transformation|SetRelativeRotation (Variables|Default|Getwatergirl_Leg) "0, 0, 0" false false)
        (Transformation|SetRelativeRotation (Variables|Default|Getwatergirl_Leg2) "0, 0, 0" false false)))))

(fn ConstructionScript)