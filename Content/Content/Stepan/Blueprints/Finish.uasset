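; Level finish trigger for either the Water or Fire character, chosen by its Type variable and labeled with that name at construction.
; On box overlap, it casts the actor to the matching character and sets a finished flag on player 0's MyPlayerState.
; The flags are crossed: Water sets FireFinished and Fire sets WaterFinished, while both print "FIRE DONE".
; The Water branch is marked temporary.
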(event OnComponentBeginOverlap(Box)
  (params (OverlappedComponent :type Primitive%20Component%20Object%20Reference) (OtherActor :type Actor%20Object%20Reference) (OtherComp :type Primitive%20Component%20Object%20Reference) (OtherBodyIndex :type Integer) (bFromSweep :type Boolean) (SweepResult :type Hit%20Result%20Structure%20%28by%20ref%29))
  (bind _returnvalue (Game|GetPlayerController 0))
  (bind _playerstate (Variables|/Script/Engine.Controller|GetPlayerState _returnvalue))
  (switch Utilities|FlowControl|Switch|SwitchonPlayerType_Enum (Variables|Default|GetType)
    (:NewEnumerator0
      (Utilities|Casting|CastToPlayerCharacter_BP_Water OtherActor)
      ;[1 0 0] TEMPORARY
      (bind _asmy_player_state (Utilities|Casting|CastToMyPlayerState _playerstate))
      (Variables|/Game/Content/Stepan/Blueprints/MyPlayerState.MyPlayerState_C|SetFireFinished? _asmy_player_state true)
      (Development|PrintString "FIRE DONE"))
    (:NewEnumerator1
      (Utilities|Casting|CastToPlayerCharacter_BP_Fire OtherActor)
      (bind _asmy_player_state_2 (Utilities|Casting|CastToMyPlayerState _playerstate))
      (Variables|/Game/Content/Stepan/Blueprints/MyPlayerState.MyPlayerState_C|SetWaterFinished? _asmy_player_state_2 true)
      (Development|PrintString "FIRE DONE"))))

(event EventBeginPlay)

(event Collision|EventActorBeginOverlap
  (params (OtherActor :type Actor%20Object%20Reference)))

(event EventTick
  (params (DeltaSeconds :type Float%20%28single-precision%29)))

(fn ConstructionScript
  (Rendering|Components|TextRender|SetText (Variables|Default|GetTextRender) (Utilities|Text|ToText(String) (Utilities|String|EnumtoString (Variables|Default|GetType)))))