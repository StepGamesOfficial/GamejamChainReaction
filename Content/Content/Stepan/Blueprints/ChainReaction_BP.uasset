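; ChainReaction_BP is an elemental trigger that marks progress on a target gate when hit by a Projectile of matching type.
; A Box overlap compares the two types, then sets WaterDone or FireDone on the Target cast to Gate_BP.
; A TextRender displays the required type.
; The construction script draws a long-lived debug line to the Target, with a self-resetting FlushPersistentLines toggle that clears and redraws it.
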(event OnComponentBeginOverlap(Box)
  (params (OverlappedComponent :type Primitive%20Component%20Object%20Reference) (OtherActor :type Actor%20Object%20Reference) (OtherComp :type Primitive%20Component%20Object%20Reference) (OtherBodyIndex :type Integer) (bFromSweep :type Boolean) (SweepResult :type Hit%20Result%20Structure%20%28by%20ref%29))
  (bind _type (Variables|Default|GetType))
  (bind _target (Variables|Default|GetTarget))
  (bind _asprojectile (Utilities|Casting|CastToProjectile OtherActor))
  (if (Utilities|Enum|Equal(Enum) _type (Variables|/Game/Content/Stepan/Blueprints/Projectile.Projectile_C|GetType _asprojectile))
    (switch Utilities|FlowControl|Switch|SwitchonPlayerType_Enum _type
      (:NewEnumerator0
        (bind _asgate_bp (Utilities|Casting|CastToGate_BP _target))
        (Variables|/Game/Content/Stepan/Blueprints/Gate_BP.Gate_BP_C|SetWaterDone? _asgate_bp true))
      (:NewEnumerator1
        (bind _asgate_bp_2 (Utilities|Casting|CastToGate_BP _target))
        (Variables|/Game/Content/Stepan/Blueprints/Gate_BP.Gate_BP_C|SetFireDone? _asgate_bp_2 true)))))

(event EventBeginPlay
  (Rendering|Components|TextRender|SetText (Variables|Default|GetTextRender) (Utilities|Text|FormatText "{type} HERE" (Utilities|Text|ToText(String) (Utilities|String|EnumtoString (Variables|Default|GetType))))))

(event Collision|EventActorBeginOverlap
  (params (OtherActor :type Actor%20Object%20Reference)))

(event EventTick
  (params (DeltaSeconds :type Float%20%28single-precision%29)))

(fn ConstructionScript
  (Rendering|Components|TextRender|SetText (Variables|Default|GetTextRender) (Utilities|Text|FormatText "{type}" (Utilities|Text|ToText(String) (Utilities|String|EnumtoString (Variables|Default|GetType)))))
  (Rendering|Debug|DrawDebugLine (Transformation|GetActorLocation) (Transformation|GetActorLocation (Variables|Default|GetTarget)) "(R=0.328616,G=0.000000,B=0.042312,A=1.000000)" 999.0 5.0 :!label _label)
  (if (Variables|Default|GetFlush%20persistent%20lines)
    (Rendering|Debug|FlushPersistentDebugLines)
    (Variables|Default|SetFlush%20persistent%20lines false)
    (goto _label)))